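; Map Blueprint that runs the last-player-standing check ending a round.
; Server-VerifPlayers counts non-spectator BP_Player actors and prints the count for debugging.
; When exactly one remains, it has each player's owning client create a win/lose widget, with spectators as losers.
; After a short delay, it calls each player's server reset for a new round.
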(event `Server - Verif Players`
  (bind _player_number (`self.Player Number`))
  (set `self.Player Number` 0)
  (bind _outactors (`GameplayStatics.GetAllActorsOfClass` "/Game/Blueprints/Player/BP_Player.BP_Player_C"))
  (for _array_element _outactors
    (if (not (`/Game/Blueprints/Player/BP_Player.Spectator` _array_element))
      (set `self.Player Number` (+ (`self.Player Number`) 1))))
  (`KismetSystemLibrary.PrintString` (`KismetStringLibrary.Conv_IntToString` _player_number))
  (if (== _player_number 1)
    (`KismetSystemLibrary.PrintString` "Good" true true (struct :`R` 1.0 :`G` 0.207055 :`A` 1.0))
    (bind _outactors_2 (`GameplayStatics.GetAllActorsOfClass` "/Game/Blueprints/Player/BP_Player.BP_Player_C"))
    (for _array_element_2 _outactors_2
      (if (`/Game/Blueprints/Player/BP_Player.Spectator` _array_element_2)
        (`/Game/Blueprints/Player/BP_Player.OWNclient - CreateWinLostWidget` _array_element_2 false)
        (else
          (`/Game/Blueprints/Player/BP_Player.OWNclient - CreateWinLostWidget` _array_element_2 true))))
    (`KismetSystemLibrary.Delay` 5.0)
    (bind _outactors_3 (`GameplayStatics.GetAllActorsOfClass` "/Game/Blueprints/Player/BP_Player.BP_Player_C"))
    (for _array_element_3 _outactors_3
      (`/Game/Blueprints/Player/BP_Player.Server - Reset Player For New Round` _array_element_3))))

(fn `UserConstructionScript`)