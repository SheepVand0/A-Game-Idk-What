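; BP_Tir is a weapon projectile that damages players it hits and rewards the shooter for kills.
; SetSettings stores the shooter, damage and an end distance, though the end distance is not used in these graphs.
; A Sphere hit calls server events that forward damage to the victim through OWNClientHit and destroy the projectile.
; If the victim's Life minus the damage reaches zero or below, the shooter receives credits.
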(event `Set Settings`
  (params (Owner :type "/Game/Blueprints/Player/BP_Player Object Reference") (Damages :type "Float (double-precision)") (`End distance` :type "Vector Structure"))
  (set `self.Player` Owner)
  (set `self.Damages` Damages)
  (set `self.End distance` `End distance`))

(event `self.Sphere.OnComponentHit`
  (params (HitComponent :type "PrimitiveComponent Object Reference") (OtherActor :type "Actor Object Reference") (OtherComp :type "PrimitiveComponent Object Reference") (NormalImpulse :type "Vector Structure") (Hit :type "HitResult Structure (by ref)"))
  (`self.Server - Hit Actions` OtherActor)
  (`self.Server - Destroy Ball`))

(event `Server - Hit Actions`
  (params (Object :type "Object Object Reference"))
  (bind _damages (`self.Damages`))
  (bind _asbp_player (cast `/Game/Blueprints/Player/BP_Player` Object))
  (`/Game/Blueprints/Player/BP_Player.OWNClient - Hit` _asbp_player _damages (`self.Player`))
  (if (<= (- (`/Game/Blueprints/Player/BP_Player.Life` _asbp_player) _damages) 0.0)
    (`/Game/Blueprints/Player/BP_Player.OWNClient - Set credits` (`self.Player`) 300 true)))

(event `Server - Destroy Ball`
  (`self.K2_DestroyActor`))

(fn `UserConstructionScript`)