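; BP_Explode is a networked explosion actor that damages players in its radius, crediting its stored owning player.
; Sphere overlaps call a server event that line-traces from the sphere toward the overlapped BP_Player on the Camera channel.
; Whichever BP_Player the trace hits takes fixed, shield-respecting damage through its owning-client damage event, so cover can block the blast.
; BeginPlay routes through server and multicast events to destroy the actor after a short delay.
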(event `OWNClient - Set Owner`
  (params (`Owning Player` :type "/Game/Blueprints/Player/BP_Player Object Reference"))
  (set `self.OwningPlayer` `Owning Player`))

(event `self.ReceiveBeginPlay`
  (`self.Server - Destroy Explosion`))

(event `Server - Destroy Explosion`
  (`self.Multicast - Destroy explosion`))

(event `self.Sphere.OnComponentBeginOverlap`
  (params (OverlappedComponent :type "PrimitiveComponent Object Reference") (OtherActor :type "Actor Object Reference") (OtherComp :type "PrimitiveComponent Object Reference") (OtherBodyIndex :type Integer) (bFromSweep :type Boolean) (SweepResult :type "HitResult Structure (by ref)"))
  (`self.Server - OverlapSettings` OtherActor))

(event `Multicast - Destroy explosion`
  (`KismetSystemLibrary.Delay` 4.0)
  (`self.K2_DestroyActor`))

(event `Server - OverlapSettings`
  (params (Object :type "Object Object Reference"))
  (bind _asbp_player (cast `/Game/Blueprints/Player/BP_Player` Object))
  (bind _outhit (`KismetSystemLibrary.LineTraceSingle` (`SceneComponent.K2_GetComponentLocation` (`self.Sphere`)) (`self.K2_GetActorLocation` _asbp_player) "TraceTypeQuery2" true))
  (bind _asbp_player_2 (cast `/Game/Blueprints/Player/BP_Player` (`.HitActor` (`GameplayStatics.BreakHitResult` _outhit))))
  (`/Game/Blueprints/Player/BP_Player.OWNClient - ApplyDamage` _asbp_player_2 75.0 false (`self.OwningPlayer`)))

(fn `UserConstructionScript`)