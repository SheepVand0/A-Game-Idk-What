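; Launcher Blueprint for the fire explosion god power, which fires the shot when a player uses it.
; OnUse stores the user through a server event, then a second server event triggers a multicast.
; The multicast spawns BP_Fire_Tir_For_Explode_Launch at the Arrow's location and rotation, ignoring collisions, and passes it the player.
; Spawning happens inside the multicast, so each machine that receives it creates its own launch actor.
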(event `/Game/Blueprints/Player/Interfaces/I_Power.On Use`
  (params (`Player Who Use` :type "/Game/Blueprints/Player/BP_Player Object Reference"))
  (`self.Server - Set Player` `Player Who Use`)
  (`self.Server - On Use`))

(event `Server - Set Player`
  (params (Player :type "/Game/Blueprints/Player/BP_Player Object Reference"))
  (set `self.Player` Player))

(event `Multicast - Spawn Tir`
  (bind _arrow (`self.Arrow`))
  (bind _returnvalue (`|SpawnActorFromClass` "/Game/Blueprints/Player/FireGodPowers/FireExplosion/BP_Fire_Tir_For_Explode_Launch.BP_Fire_Tir_For_Explode_Launch_C" (`KismetMathLibrary.MakeTransform` (`SceneComponent.K2_GetComponentLocation` _arrow) (`SceneComponent.K2_GetComponentRotation` _arrow)) "AlwaysSpawn" "OverrideRootScale" null null))
  (`/Game/Blueprints/Player/FireGodPowers/FireExplosion/BP_Fire_Tir_For_Explode_Launch.Server - Set Player` _returnvalue (`self.Player`)))

(event `Server - On Use`
  (`self.Multicast - Spawn Tir`))

(fn `UserConstructionScript`
  (`parent.UserConstructionScript`))