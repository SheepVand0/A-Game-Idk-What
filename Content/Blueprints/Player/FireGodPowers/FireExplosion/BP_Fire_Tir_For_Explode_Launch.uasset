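; Fire God power projectile that triggers an explosion when its sphere hits something.
; The hit calls a server event, which relays to a multicast that spawns BP_Explode at the projectile's location with random yaw.
; Each explosion receives the stored Player through its set-owner call, with that reference assigned by a separate server event.
; The graph does not destroy the projectile after impact.
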(event `self.Sphere.OnComponentHit`
  (params (HitComponent :type "PrimitiveComponent Object Reference") (OtherActor :type "Actor Object Reference") (OtherComp :type "PrimitiveComponent Object Reference") (NormalImpulse :type "Vector Structure") (Hit :type "HitResult Structure (by ref)"))
  (`self.Server - Hit`))

(event `Server - Hit`
  (`self.Multicast - Hit`))

(event `Multicast - Hit`
  (bind _returnvalue (`|SpawnActorFromClass` "/Game/Blueprints/Player/BP_Explode.BP_Explode_C" (`KismetMathLibrary.MakeTransform` (`self.K2_GetActorLocation`) (`KismetMathLibrary.MakeRotator` 0.0 0.0 (`KismetMathLibrary.RandomFloatInRange` 0.0 360.0))) "Undefined" "OverrideRootScale" null null))
  (`/Game/Blueprints/Player/BP_Explode.OWNClient - Set Owner` _returnvalue (`self.Player`)))

(event `Server - Set Player`
  (params (Player :type "/Game/Blueprints/Player/BP_Player Object Reference"))
  (set `self.Player` Player))

(fn `UserConstructionScript`
  (`parent.UserConstructionScript`))