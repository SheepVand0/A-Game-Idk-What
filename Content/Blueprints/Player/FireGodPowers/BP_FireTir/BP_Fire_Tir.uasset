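; Fire God power actor that fires a shot by spawning a BP_Fire_Tir_Launch when used.
; OnUse passes the using player through a server event, then calls a second server event that multicasts the shot.
; The multicast spawns the launch actor at StartLoc's world location and rotation on each machine it reaches, then calls its OnUse with the stored Player.
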(event `/Game/Blueprints/Player/Interfaces/I_Power.On Use`
  (params (`Player Who Use` :type "/Game/Blueprints/Player/BP_Player Object Reference"))
  (`self.Server - Set Player` `Player Who Use`)
  (`self.Server - On Use`))

(event `Server - Set Player`
  (params (Player :type "/Game/Blueprints/Player/BP_Player Object Reference"))
  (set `self.Player` Player))

(event `Server - On Use`
  (`self.Multicast - On Use`))

(event `Multicast - On Use`
  (bind _startloc (`self.StartLoc`))
  (bind _returnvalue (`|SpawnActorFromClass` "/Game/Blueprints/Player/FireGodPowers/BP_FireTir/BP_Fire_Tir_Launch.BP_Fire_Tir_Launch_C" (`KismetMathLibrary.MakeTransform` (`SceneComponent.K2_GetComponentLocation` _startloc) (`SceneComponent.K2_GetComponentRotation` _startloc)) "AlwaysSpawn" "OverrideRootScale" null null))
  (`/Game/Blueprints/Player/Interfaces/I_Power.On Use` _returnvalue (`self.Player`)))

(fn `UserConstructionScript`
  (`parent.UserConstructionScript`))